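; BP_FinalDoor is an interactable double door in the Medieval Dungeon that opens only when the player character holds a key.
; On Interact it casts the player to BP_FirstPersonCharacter and checks HaveKey, playing a locked sound at the doorway without one.
; With the key, a FlipFlop alternates opening and closing sounds while playing or reversing a Timeline that swings both leaves outward in mirrored yaw.
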(event `/Game/MedievalDungeon/Interact_Interface.Interact`
  (bind _returnvalue (`SceneComponent.K2_GetComponentLocation` (`self.SM_DoorWay`)))
  ;[0.6354 1 0.6772] Open Door
  (if (`/Game/FirstPerson/Blueprints/BP_FirstPersonCharacter.HaveKey` (cast `/Game/FirstPerson/Blueprints/BP_FirstPersonCharacter` (`GameplayStatics.GetPlayerCharacter` 0) :!pure true))
    (`/Engine/EditorBlueprintResources/StandardMacros.FlipFlop`
      (:`A`
        (`GameplayStatics.PlaySoundAtLocation` "/Game/Sounds/Objects/Door_Wood_Open_01.Door_Wood_Open_01" _returnvalue (struct) 1.0 1.0 0.0 null null null null)
        (bind (_direction _newtrack_0) (`Timeline|Timeline` :!label _label)
          (:`Update`
            (`SceneComponent.K2_SetRelativeRotation` (`self.SM_DoorWay_Large_Door_Left`) (`KismetMathLibrary.MakeRotator` 0.0 0.0 (`KismetMathLibrary.Lerp` 0.0 -90.0 _newtrack_0)) false false)
            (`SceneComponent.K2_SetRelativeRotation` (`self.SM_DoorWay_Large_Door_Right`) (`KismetMathLibrary.MakeRotator` 0.0 0.0 (`KismetMathLibrary.Lerp` 0.0 90.0 _newtrack_0)) false false))))
      (:`B`
        (`GameplayStatics.PlaySoundAtLocation` "/Game/Sounds/Objects/Door_Wood_Close_01.Door_Wood_Close_01" _returnvalue (struct) 1.0 1.0 0.0 null null null null)
        (goto _label :!via `Reverse`)))
    (else
      (`GameplayStatics.PlaySoundAtLocation` "/Game/Sounds/Objects/Door_Wood_Locked.Door_Wood_Locked" _returnvalue (struct) 1.0 1.0 0.0 null null null null))))

(fn `UserConstructionScript`)